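; BP_P38 is a player-controlled P-38 aircraft that constantly flies forward and fires rockets.
; Tick spins both propeller meshes and feeds full movement input along the actor's forward vector.
; Mouse axes rotate the actor locally, scaled by RotateSpeed and delta time: up/down pitches, while left/right rolls rather than yaws.
; Left mouse button spawns a BP_Rocket at the RocketLaunch component's world transform.
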(event EventBeginPlay)

(event Collision|EventActorBeginOverlap
  (params (OtherActor :type Actor%20Object%20Reference)))

(event EventTick
  (params (DeltaSeconds :type Float%20%28single-precision%29))
  (Utilities|FlowControl|Sequence
    (:then_0
      (Transformation|AddLocalRotation (Variables|Default|GetSM_P38_PropellerLeft) (Math|Rotator|MakeRotator (* DeltaSeconds 1e+04) 0.0 0.0) false false))
    (:then_1
      (Transformation|AddLocalRotation (Variables|Default|GetSM_P38_PropellerRight) (Math|Rotator|MakeRotator (* DeltaSeconds 1e+04) 0.0 0.0) false false))
    (:then_2
      (Pawn|Input|AddMovementInput (Transformation|GetActorForwardVector) 1.0 false))))

(event Input|AxisEvents|InputAxisLookUp/DownMouse
  (params (AxisValue :type Float%20%28single-precision%29))
  (Transformation|AddActorLocalRotation (Math|Rotator|MakeRotator 0.0 (* AxisValue (Variables|Default|GetRotateSpeed) (Utilities|Time|GetWorldDeltaSeconds)) 0.0) false false))

(event Input|AxisEvents|InputAxisTurnRight/LeftMouse
  (params (AxisValue :type Float%20%28single-precision%29))
  (Transformation|AddActorLocalRotation (Math|Rotator|MakeRotator (* (Variables|Default|GetRotateSpeed) (Utilities|Time|GetWorldDeltaSeconds) AxisValue) 0.0 0.0) false false))

(event Input|MouseEvents|LeftMouseButton
  (params (Key :type Key%20Structure :default "None"))
  (:Pressed
    (Game|SpawnActorfromClass "/Game/Blueprints/BP_Rocket.BP_Rocket_C" (Transformation|GetSocketTransform (Variables|Default|GetRocketLaunch) "None" "RTS_World") "Undefined" "MultiplyWithRoot" 0 0)))

(fn ConstructionScript)